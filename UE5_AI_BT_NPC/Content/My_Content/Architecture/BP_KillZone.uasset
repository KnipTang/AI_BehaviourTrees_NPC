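; BP_KillZone is a trigger volume that removes NPCs that enter it while the player's simulation is active.
; When its Cube component is overlapped, it finds BP_Player in the world and checks its IsSimulating flag.
; If the flag is set and the overlapping actor is a CPP_NPC, it prints the name, calls Finished with false, then destroys that actor.
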(event `self.Cube.OnComponentBeginOverlap`
  (params (OverlappedComponent :type "PrimitiveComponent Object Reference") (OtherActor :type "Actor Object Reference") (OtherComp :type "PrimitiveComponent Object Reference") (OtherBodyIndex :type Integer) (bFromSweep :type Boolean) (SweepResult :type "HitResult Structure (by ref)"))
  (bind _returnvalue (`GameplayStatics.GetActorOfClass` "/Game/My_Content/Player/BP_Player.BP_Player_C"))
  (if (`/Game/My_Content/Player/BP_Player.IsSimulating` _returnvalue)
    (if (`GameplayStatics.ObjectIsA` OtherActor "/Script/UE5_AI_BT_NPC.CPP_NPC")
      (`KismetSystemLibrary.PrintString` (`KismetStringLibrary.Concat_StrStr` "NPC DESTROYED: " (`KismetSystemLibrary.GetDisplayName` OtherActor)))
      (bind _ascpp_npc (cast `CPP_NPC` OtherActor))
      (`CPP_NPC.Finished` _ascpp_npc false)
      (`self.K2_DestroyActor` OtherActor))))

(fn `UserConstructionScript`)