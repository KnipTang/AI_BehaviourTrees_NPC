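; Base NPC Blueprint that continually adjusts its roll to follow the slope of the ground beneath it.
; Every Tick, XRotateNPC casts two downward-angled visibility traces toward the actor's right and left and compares their hit distances.
; It nudges roll one fixed step toward the farther hit, with no dead zone or delta-time scaling.
; Debug lines always draw; the MDriving/DebugLines branch is empty.
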(event `self.ReceiveBeginPlay`)

(event `self.ReceiveTick`
  (params (DeltaSeconds :type "Float (single-precision)"))
  (`self.XRotateNPC`)
  (if (or (`self.m_Driving`) (`self.debugLines`))
    _))

(fn `UserConstructionScript`)

(fn `XRotateNPC`
  (locals (NewLocalVar :type Boolean) (Offset :type Integer :default 500) (`Out Hit Distance` :type "Float (single-precision)" :default 0.0) (`Out Hit Distance_0` :type "Float (single-precision)" :default 0.0))
  (bind (_returnvalue_x _returnvalue_y _returnvalue_z) (`KismetMathLibrary.BreakVector` (`self.K2_GetActorLocation`)))
  (bind (_returnvalue_x_2 _returnvalue_y_2 _returnvalue_z_2) (`KismetMathLibrary.BreakVector` (`self.K2_GetActorLocation`)))
  (bind (_returnvalue_roll _returnvalue_pitch _returnvalue_yaw) (`KismetMathLibrary.BreakRotator` (`self.K2_GetActorRotation`)))
  (bind (_returnvalue_x_3 _returnvalue_y_3 _returnvalue_z_3) (`KismetMathLibrary.BreakVector` (+ (* (`local.Offset`) (`self.GetActorRightVector`)) (`self.K2_GetActorLocation`))))
  (bind (_returnvalue_x_4 _returnvalue_y_4 _returnvalue_z_4) (`KismetMathLibrary.BreakVector` (+ (* (* (`local.Offset`) -1) (`self.GetActorRightVector`)) (`self.K2_GetActorLocation`))))
  (bind _outhit (`KismetSystemLibrary.LineTraceSingle` (`KismetMathLibrary.MakeVector` _returnvalue_x_2 _returnvalue_y_2 _returnvalue_z_2) (`KismetMathLibrary.MakeVector` _returnvalue_x_3 _returnvalue_y_3 (+ _returnvalue_z_3 -500.0)) "TraceTypeQuery1"))
  (set `local.Out Hit Distance` (`.Distance` (`GameplayStatics.BreakHitResult` _outhit)))
  (`KismetSystemLibrary.DrawDebugLine` (`.TraceStart` (`GameplayStatics.BreakHitResult` _outhit)) (`.TraceEnd` (`GameplayStatics.BreakHitResult` _outhit)) (struct :`R` 1.0 :`G` 0.090769 :`B` 0.88555 :`A` 1.0) 0.1)
  (bind _outhit_2 (`KismetSystemLibrary.LineTraceSingle` (`KismetMathLibrary.MakeVector` _returnvalue_x _returnvalue_y _returnvalue_z) (`KismetMathLibrary.MakeVector` _returnvalue_x_4 _returnvalue_y_4 (+ _returnvalue_z_4 -500.0)) "TraceTypeQuery1"))
  (set `local.Out Hit Distance_0` (`.Distance` (`GameplayStatics.BreakHitResult` _outhit_2)))
  (`KismetSystemLibrary.DrawDebugLine` (`.TraceStart` (`GameplayStatics.BreakHitResult` _outhit_2)) (`.ImpactPoint` (`GameplayStatics.BreakHitResult` _outhit_2)) (struct :`R` 1.0 :`G` 0.090769 :`B` 0.88555 :`A` 1.0) 0.1)
  (if (> (`local.Out Hit Distance`) (`local.Out Hit Distance_0`))
    (`self.K2_SetActorRotation` (`KismetMathLibrary.MakeRotator` (+ _returnvalue_roll 1.0) _returnvalue_pitch _returnvalue_yaw))
    (else
      (`self.K2_SetActorRotation` (`KismetMathLibrary.MakeRotator` (+ _returnvalue_roll -1.0) _returnvalue_pitch _returnvalue_yaw)))))