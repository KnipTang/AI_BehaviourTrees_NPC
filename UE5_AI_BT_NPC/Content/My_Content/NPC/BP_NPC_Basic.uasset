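; Basic NPC driver that sets its type to Basic2Lines and caches the spline of the BP_Road actor on BeginPlay.
; While driving or with debug lines enabled, Tick calls XRotateNPC, then computes left and right ray endpoints.
; Each ray angles forward, sideways and downward from the actor, shaped by a down-ray multiplier and ray length; no trace happens in this graph.
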(event `self.ReceiveBeginPlay`
  (`self.SetNPCType` "Basic2Lines")
  (bind _returnvalue (`GameplayStatics.GetActorOfClass` "/Game/My_Content/Architecture/BP_Road.BP_Road_C"))
  (set `self.m_Spline` (`/Game/My_Content/Architecture/BP_Road.Spline` _returnvalue)))

(event `self.ReceiveTick`
  (params (DeltaSeconds :type "Float (single-precision)"))
  (if (or (`self.m_Driving`) (`self.debugLines`))
    (`self.XRotateNPC`)
    (bind _output_get (set `self.LeftDownwardVector` (+ (* (+ (* (`self.GetActorRightVector`) -1.0) (`self.GetActorForwardVector`)) (* (`self.m_DownRayMultiplier`) 10.0)) (* (`self.GetActorUpVector`) -1.0))))
    (set `self.m_EndLeftRay` (+ (`self.K2_GetActorLocation`) (* _output_get (`self.m_RayLength`))))
    (bind _output_get_2 (set `self.RightDownwardVector` (+ (* (+ (`self.GetActorRightVector`) (`self.GetActorForwardVector`)) (* (`self.m_DownRayMultiplier`) 10.0)) (* (`self.GetActorUpVector`) -1.0))))
    (set `self.m_EndRightRay` (+ (`self.K2_GetActorLocation`) (* _output_get_2 (`self.m_RayLength`))))))

(fn `UserConstructionScript`)