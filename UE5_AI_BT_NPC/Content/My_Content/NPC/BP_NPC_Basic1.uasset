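; BP_NPC_Basic1 is a driving NPC that configures itself as the Basic2Lines type on BeginPlay.
; Each tick it calls XRotateNPC, then, while driving or showing debug lines, recomputes left and right ray endpoints.
; Both rays angle slightly downward to either side of a point ahead of the actor, scaled by MRayLength.
; The graph only computes these endpoints and performs no traces itself.
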(event `self.ReceiveBeginPlay`
  (`self.SetNPCType` "Basic2Lines"))

(event `self.ReceiveTick`
  (params (DeltaSeconds :type "Float (single-precision)"))
  (`self.XRotateNPC`)
  (if (or (`self.m_Driving`) (`self.debugLines`))
    (set `self.LeftDownwardVector` (+ (* (`self.GetActorRightVector`) -1.0) (* (`KismetMathLibrary.Vector_Down`) 0.3)))
    (set `self.m_EndLeftRay` (+ (+ (`self.K2_GetActorLocation`) (* (`self.GetActorForwardVector`) 500.0)) (* (`self.LeftDownwardVector`) (`self.m_RayLength`))))
    (set `self.RightDownwardVector` (+ (* (`self.GetActorRightVector`) 1.0) (* (`KismetMathLibrary.Vector_Down`) 0.3)))
    (set `self.m_EndRightRay` (+ (+ (`self.K2_GetActorLocation`) (* (`self.GetActorForwardVector`) 500.0)) (* (`self.RightDownwardVector`) (`self.m_RayLength`))))))

(fn `UserConstructionScript`)