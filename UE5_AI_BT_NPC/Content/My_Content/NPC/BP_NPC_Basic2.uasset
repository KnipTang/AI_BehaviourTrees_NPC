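; BP_NPC_Basic2 is an NPC variant that registers itself as the Basic2Lines type on BeginPlay.
; Each Tick it calls XRotateNPC, then, while driving or showing debug lines, computes end points for a left and a right sensing ray.
; Both rays reach ahead of the actor and angle sideways and downward, scaled by MRayLength.
; The graph only stores these end points and performs no trace itself.
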(event `self.ReceiveBeginPlay`
  (`self.SetNPCType` "Basic2Lines"))

(event `self.ReceiveTick`
  (params (DeltaSeconds :type "Float (single-precision)"))
  (`self.XRotateNPC`)
  (if (or (`self.m_Driving`) (`self.debugLines`))
    (set `self.LeftDownwardVector` (`KismetMathLibrary.Normal` (+ (* (`self.GetActorRightVector`) -1.0) (* (`KismetMathLibrary.Vector_Down`) 0.7))))
    (set `self.m_EndLeftRay` (+ (+ (`self.K2_GetActorLocation`) (* (`self.GetActorForwardVector`) (`self.m_RayLength`))) (* (`self.LeftDownwardVector`) (`self.m_RayLength`))))
    (set `self.RightDownwardVector` (`KismetMathLibrary.Normal` (+ (* (`self.GetActorRightVector`) 1.0) (* (`KismetMathLibrary.Vector_Down`) 0.7))))
    (set `self.m_EndRightRay` (+ (+ (`self.K2_GetActorLocation`) (* (`self.GetActorForwardVector`) (`self.m_RayLength`))) (* (`self.RightDownwardVector`) (`self.m_RayLength`))))))

(fn `UserConstructionScript`)