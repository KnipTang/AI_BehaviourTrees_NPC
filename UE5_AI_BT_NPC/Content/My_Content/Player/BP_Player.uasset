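; BP_Player is the player Blueprint, forwarding movement and mouse-look axis inputs to movement, turn and look functions.
; Hard-wired keys act as test controls over NPCs found with GetAllActorsOfClass.
; H toggles debug lines on every CPP_NPC, and Y calls StartDriving on them.
; F moves the player to the first BP_NPC_Basic's horizontal position while keeping the player's own height.
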(event EventBeginPlay)

(event Collision|EventActorBeginOverlap
  (params (OtherActor :type Actor%20Object%20Reference)))

(event EventTick
  (params (DeltaSeconds :type Float%20%28single-precision%29)))

(event Input|AxisEvents|InputAxisMoveForward/Backward
  (params (AxisValue :type Float%20%28single-precision%29))
  (Class|CPPMainPlayer|MovForward AxisValue))

(event Input|AxisEvents|InputAxisMoveRight/Left
  (params (AxisValue :type Float%20%28single-precision%29))
  (Class|CPPMainPlayer|MovRight AxisValue))

(event Input|AxisEvents|InputAxisLookUp/DownMouse
  (params (AxisValue :type Float%20%28single-precision%29))
  (Class|CPPMainPlayer|LookUp AxisValue))

(event Input|AxisEvents|InputAxisTurnRight/LeftMouse
  (params (AxisValue :type Float%20%28single-precision%29))
  (Class|CPPMainPlayer|Turn AxisValue))

(event Input|KeyboardEvents|DebugKeyH
  (params (Key :type Key%20Structure :default "None") (ActionValue :type Input%20Action%20Value%20Structure))
  (:Pressed
    (bind _outactors (Actor|GetAllActorsOfClass "/Script/UE5_AI_BT_NPC.CPP_NPC"))
    (for _array_element _outactors
      (Variables|/Script/UE5_AI_BT_NPC.CPP_NPC|SetdebugLines _array_element (not (Variables|/Script/UE5_AI_BT_NPC.CPP_NPC|GetdebugLines _array_element))))))

(event Input|KeyboardEvents|Y
  (params (Key :type Key%20Structure :default "None"))
  (:Pressed
    (bind _outactors (Actor|GetAllActorsOfClass "/Script/UE5_AI_BT_NPC.CPP_NPC"))
    (Class|CPPNPC|StartDriving _outactors)))

(event Input|KeyboardEvents|F
  (params (Key :type Key%20Structure :default "None"))
  (:Pressed
    (bind _outactors (Actor|GetAllActorsOfClass "/Game/My_Content/NPC/BP_NPC_Basic.BP_NPC_Basic_C"))
    (Transformation|SetActorLocation (Math|Vector|MakeVector (.x (Transformation|GetActorLocation (Utilities|Array|Get(acopy) _outactors))) (.y (Transformation|GetActorLocation (Utilities|Array|Get(acopy) _outactors))) (.z (Transformation|GetActorLocation))) false false)))

(fn ConstructionScript)